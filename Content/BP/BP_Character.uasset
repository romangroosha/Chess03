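; Grid-based player character that starts at the board's center and moves on BP_PlayerController move-button events.
; A line trace checks for a non-empty BP_Square, then timelines lerp position and cylinder yaw, or only yaw when blocked.
; After each move it derives facing, traces surrounding squares, lights three by direction, and lights and flags the fourth if those are empty.
; It also triggers camera obstacle rotation; clamped HP helpers exist but are unwired.
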(event `self.ReceiveBeginPlay`
  (bind (_center_x _center_y) (`KismetMathLibrary.BreakVector2D` (`/Game/BP/BP_Board.CenterOfBoard` (`self.Board_Ref`))))
  (`self.Set_Board_Ref`)
  (`self.Set_PlayerController_Ref`)
  (`self.Set_Camera_Ref`)
  (`self.Set_AI_Enemy_Ref`)
  (add `/Game/BP/BP_PlayerController.MoveButtonsEvent` (`self.PlayerController_Ref`) (`|CreateDelegate` :!event `Move Buttons Event`))
  (`self.K2_SetActorLocation` (`KismetMathLibrary.MakeVector` _center_x _center_y 100.0)) ; Start in Center
  (`self.Set_CameraStartLocation`)
  (`KismetSystemLibrary.Delay` 0.1)
  (`self.LT Availiable Moves`))

(event `Move Buttons Event`
  (params (x :type "Float (double-precision)") (y :type "Float (double-precision)") (`Rotation Yaw` :type "Float (double-precision)") (Index :type Integer))
  (`self.Set_MoveVariables` x y `Rotation Yaw` Index)
  (if (`self.IsMoveFinished`)
    (set `self.IsMoveFinished` false)
    (bind _bool (`self.LT_Move`)) ; Can move?
    (if _bool
      (`self.Set_MoveUtilityVariables` (`self.CharacterCylinder`)) ; Rotation of Target, Location Actor
      (bind (_direction _0_to_1) (`Timeline|Timeline_2` :!via `PlayFromStart`)
        (:`Update`
          (set `self.IsMoveFinished` false)
          (`self.LerpLocation_Move` _0_to_1)
          (`self.LerpRotation_Move` _0_to_1 (`self.CharacterCylinder`)))
        (:`Finished`
          (set `self.IsMoveFinished` true)
          (`self.WhichDirectionCharIsLooking_Move` (`self.CharacterCylinder`) :!pinned true :!label _label) ; Find Direction
          (`self.LT Availiable Moves`)
          (`/Game/BP/BP_Camera.ObstacleRotationEvent` (`self.Camera_Ref`))))
      (else
        (`self.Set_MoveUtilityVariables` (`self.CharacterCylinder`)) ; Rotation of Target, Location Actor
        (bind (_direction_2 _0_to_1_2) (`Timeline|Timeline_1` :!via `PlayFromStart`)
          (:`Update`
            (set `self.IsMoveFinished` false)
            (`self.LerpRotation_Move` _0_to_1_2 (`self.CharacterCylinder`)))
          (:`Finished`
            (set `self.IsMoveFinished` true)
            (goto _label)))))))

(fn `LerpLocation_Move`
  (params (Alpha :type "Float (double-precision)"))
  (locals (NewLocalVar_0 :type "Vector Structure") (NewLocalVar_1 :type "Vector Structure"))
  (`self.K2_SetActorLocation` (`KismetMathLibrary.VLerp` (`self.Move_Location 1`) (`self.Move_Location 2`) Alpha)))

(fn `LerpRotation_Move`
  (params (Alpha :type "Float (double-precision)") (`Set Target` :type "SceneComponent Object Reference"))
  (locals (Set_Target_Local :type "SceneComponent Object Reference"))
  (set `local.Set_Target_Local` `Set Target`)
  (if (!= (`self.Move_Rotation 1`) (`self.Move_Rotation 2`))
    (if (and (or (== (`self.Move_Rotation 1`) 180.0) (== (`self.Move_Rotation 1`) 135.0)) (`KismetMathLibrary.InRange_FloatFloat` (`self.Move_Rotation 2`) -135.0 -45.0))
      (set `self.Move_Rotation 2` (+ (`self.Move_Rotation 2`) 360.0))
      (elif (and (`KismetMathLibrary.InRange_FloatFloat` (`self.Move_Rotation 1`) -135.0 -45.0) (or (== (`self.Move_Rotation 2`) 180.0) (== (`self.Move_Rotation 2`) 135.0)))
        (set `self.Move_Rotation 2` (- (`self.Move_Rotation 2`) 360.0))))
    (`SceneComponent.K2_SetWorldRotation` (`local.Set_Target_Local`) (`KismetMathLibrary.MakeRotator` 0.0 0.0 (`KismetMathLibrary.Lerp` (`self.Move_Rotation 1`) (`self.Move_Rotation 2`) Alpha)) false false)))

(fn `LT Availiable Moves`
  (locals (ObjectTypes :type "Array of EObjectTypeQuery Enum"))
  (`|ExecutionSequence`
    (:`then_0`
      (set `self.R_Blocked` false)
      (set `self.U_Blocked` false)
      (set `self.L_Blocked` false)
      (set `self.D_Blocked` false))
    (:`then_1`
      (`KismetArrayLibrary.Array_Clear` (`self.ActorsAround`))
      (for _array_element (`self.LocationsAround`)
        (bind (_outhit _returnvalue) (`KismetSystemLibrary.LineTraceSingleForObjects` :`Start` (`SceneComponent.K2_GetComponentLocation` (`self.LT_Sphere`)) :`End` (+ (`KismetMathLibrary.MakeVector` (`KismetMathLibrary.BreakVector2D` _array_element) (`.Y` (`KismetMathLibrary.BreakVector2D` _array_element)) -25.0) (`self.K2_GetActorLocation`)) :`ObjectTypes` (`local.ObjectTypes`) :`TraceColor` (struct :`R` 1.0 :`G` 0.503061 :`A` 1.0)))
        (if _returnvalue
          (`KismetArrayLibrary.Array_Add` (`self.ActorsAround`) (`.HitActor` (`GameplayStatics.BreakHitResult` _outhit))))))
    (:`then_2`
      (if (== (`self.Move_Direction`) "D")
        (bind _ischarblocked (`self.LightSquaresAroundByIndex` 0 2 6))
        (if _ischarblocked
          (message `/Game/BP/Interfaces/Interface_LightSquare.Interface_LightSquareOnHit` (`|GetArrayItem` (`self.ActorsAround`) 4))
          (set `self.D_Blocked` true))))
    (:`then_3`
      (if (== (`self.Move_Direction`) "L")
        (bind _ischarblocked_2 (`self.LightSquaresAroundByIndex` 0 2 4))
        (if _ischarblocked_2
          (message `/Game/BP/Interfaces/Interface_LightSquare.Interface_LightSquareOnHit` (`|GetArrayItem` (`self.ActorsAround`) 6))
          (set `self.L_Blocked` true))))
    (:`then_4`
      (if (== (`self.Move_Direction`) "U")
        (bind _ischarblocked_3 (`self.LightSquaresAroundByIndex` 2 4 6))
        (if _ischarblocked_3
          (message `/Game/BP/Interfaces/Interface_LightSquare.Interface_LightSquareOnHit` (`|GetArrayItem` (`self.ActorsAround`)))
          (set `self.U_Blocked` true))))
    (:`then_5`
      (if (== (`self.Move_Direction`) "R")
        (bind _ischarblocked_4 (`self.LightSquaresAroundByIndex` 0 4 6))
        (if _ischarblocked_4
          (message `/Game/BP/Interfaces/Interface_LightSquare.Interface_LightSquareOnHit` (`|GetArrayItem` (`self.ActorsAround`) 2))
          (set `self.R_Blocked` true))))))

(fn `LT_Move`
  (returns (Bool :type Boolean))
  (locals (X_Local :type "Float (double-precision)") (Y_Local :type "Float (double-precision)") (IndexRotation_Local :type "Float (double-precision)") (ObjectTypes_Local :type "Array of EObjectTypeQuery Enum"))
  (bind _outhit (`KismetSystemLibrary.LineTraceSingleForObjects` (`SceneComponent.K2_GetComponentLocation` (`self.LT_Sphere`)) (+ (`KismetMathLibrary.MakeVector` (`self.Move_X`) (`self.Move_Y`) -25.0) (`self.K2_GetActorLocation`)) (`local.ObjectTypes_Local`))) ; Line Traces from LT_Sphere to Move Location
  (return (and (`KismetMathLibrary.ClassIsChildOf` (`GameplayStatics.GetObjectClass` (`.HitActor` (`GameplayStatics.BreakHitResult` _outhit))) "/Game/BP/BP_Square.BP_Square_C") (!= (`GameplayStatics.GetObjectClass` (`.HitActor` (`GameplayStatics.BreakHitResult` _outhit))) "/Game/BP/Square/BP_Square_Empty.BP_Square_Empty_C"))))

(fn `Minus_HP`
  (params (Minus :type "Float (double-precision)"))
  (bind (_maxandmin_hp_x _maxandmin_hp_y) (`KismetMathLibrary.BreakVector2D` (`self.MaxAndMin_HP`)))
  (set `self.Current_HP` (`KismetMathLibrary.FClamp` (- (`self.Current_HP`) Minus) _maxandmin_hp_x _maxandmin_hp_y)))

(fn `Plus_HP`
  (params (Plus :type "Float (double-precision)"))
  (bind (_maxandmin_hp_x _maxandmin_hp_y) (`KismetMathLibrary.BreakVector2D` (`self.MaxAndMin_HP`)))
  (set `self.Current_HP` (`KismetMathLibrary.FClamp` (+ (`self.Current_HP`) Plus) _maxandmin_hp_x _maxandmin_hp_y)))

(fn `Set_AI_Enemy_Ref`
  (`/Engine/EditorBlueprintResources/StandardMacros.IsValid` (`self.AI_Enemy_Ref`)
    (:`Is Not Valid`
      (bind _returnvalue (`GameplayStatics.GetActorOfClass` "/Game/BP/BP_AI_Enemy.BP_AI_Enemy_C"))
      (set `self.AI_Enemy_Ref` _returnvalue))))

(fn `Set_Board_Ref`
  (`/Engine/EditorBlueprintResources/StandardMacros.IsValid` (`self.Board_Ref`)
    (:`Is Not Valid`
      (bind _returnvalue (`GameplayStatics.GetActorOfClass` "/Game/BP/BP_Board.BP_Board_C"))
      (set `self.Board_Ref` _returnvalue))))

(fn `Set_Camera_Ref`
  (`/Engine/EditorBlueprintResources/StandardMacros.IsValid` (`self.Camera_Ref`)
    (:`Is Not Valid`
      (bind _returnvalue (`GameplayStatics.GetActorOfClass` "/Game/BP/BP_Camera.BP_Camera_C"))
      (set `self.Camera_Ref` _returnvalue))))

(fn `Set_CameraStartLocation`
  (locals (`Save Camera Lag Status` :type Boolean))
  (set `local.Save Camera Lag Status` (`SpringArmComponent.bEnableCameraLag` (`/Game/BP/BP_Camera.SpringArm` (`self.Camera_Ref`))))
  (set `SpringArmComponent.bEnableCameraLag` false (`/Game/BP/BP_Camera.SpringArm` (`self.Camera_Ref`)))
  (`self.K2_SetActorLocation` (`self.Camera_Ref`) (`KismetMathLibrary.MakeVector` (- (.x (`self.K2_GetActorLocation`)) 400.0) (.y (`self.K2_GetActorLocation`)) (+ (.z (`self.K2_GetActorLocation`)) 1000.0)) false false) ; Set Start Location
  (set `SpringArmComponent.bEnableCameraLag` (`local.Save Camera Lag Status`) (`/Game/BP/BP_Camera.SpringArm` (`self.Camera_Ref`))))

(fn `Set_MoveUtilityVariables`
  (params (`Set Target` :type "SceneComponent Object Reference"))
  (bind _returnvalue (`self.K2_GetActorLocation`))
  (bind (_returnvalue_roll _returnvalue_pitch _returnvalue_yaw) (`KismetMathLibrary.BreakRotator` (`SceneComponent.K2_GetComponentRotation` `Set Target`)))
  (set `self.Move_Location 1` _returnvalue)
  (set `self.Move_Location 2` (+ (`KismetMathLibrary.MakeVector` (`self.Move_X`) (`self.Move_Y`)) _returnvalue))
  (set `self.Move_Rotation 1` _returnvalue_yaw)
  (set `self.Move_Rotation 2` (`self.Move_Rotation Yaw`)))

(fn `Set_MoveVariables`
  (params (x :type "Float (double-precision)") (y :type "Float (double-precision)") (`Rotation Yaw` :type "Float (double-precision)") (index :type Integer))
  (set `self.Move_X` x)
  (set `self.Move_Y` y)
  (set `self.Move_Rotation Yaw` `Rotation Yaw`)
  (set `self.Move_Index` index))

(fn `Set_PlayerController_Ref`
  (`/Engine/EditorBlueprintResources/StandardMacros.IsValid` (`self.PlayerController_Ref`)
    (:`Is Not Valid`
      (bind _asbp_player_controller (cast `/Game/BP/BP_PlayerController` (`GameplayStatics.GetPlayerController` 0)))
      (set `self.PlayerController_Ref` _asbp_player_controller))))

(fn `UserConstructionScript`)

(fn `WhichDirectionCharIsLooking_Move`
  (params (`Set Target` :type "StaticMeshComponent Object Reference"))
  (locals (SetTarget_Local :type "StaticMeshComponent Object Reference"))
  (set `local.SetTarget_Local` `Set Target`)
  (bind _keys (`BlueprintMapLibrary.Map_Keys` (`self.Move_DirectionMap`)))
  (for _array_element _keys
    (if (== _array_element (`SceneComponent.GetForwardVector` (`local.SetTarget_Local`)) :`ErrorTolerance` 0.1)
      (set `self.Move_Direction` (`BlueprintMapLibrary.Map_Find` (`self.Move_DirectionMap`) _array_element))
      (break)))
  (return))