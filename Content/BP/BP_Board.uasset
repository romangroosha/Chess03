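; BP_Board procedurally builds a square grid board from child actor tiles and populates it with AI enemies.
; The construction script makes borders empty, with layered random checks scattering further empty squares toward the edges for a ragged outline.
; Other squares randomly become regular or damage tiles, occasionally with a pickable, buff or debuff, and are stored in an array.
; BeginPlay spawns enemies using X and Y drawn independently from that array.
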(event `self.ReceiveBeginPlay`
  (bind (_output_x _output_y) (`KismetMathLibrary.BreakVector2D` (`|GetArrayItem` (`self.NotEmptySquaresArray`) (`KismetMathLibrary.RandomIntegerInRange` 0 (`KismetArrayLibrary.Array_LastIndex` (`self.NotEmptySquaresArray`))))))
  (`KismetSystemLibrary.PrintString` (`KismetStringLibrary.Conv_IntToString` (`KismetArrayLibrary.Array_LastIndex` (`self.NotEmptySquaresArray`))) true true (struct :`G` 1.0 :`B` 0.324123 :`A` 1.0) 5.0)
  (for _ (range 5)
    (`|SpawnActorFromClass` "/Game/BP/BP_AI_Enemy.BP_AI_Enemy_C" (`KismetMathLibrary.MakeTransform` (`KismetMathLibrary.MakeVector` _output_x _output_y 20.0)) "Undefined" "OverrideRootScale" null null)))

(fn `CenterOfBoard`
  (returns (Center :type "Vector2D Structure"))
  (return (`KismetMathLibrary.MakeVector2D` (`KismetMathLibrary.Conv_IntToDouble` (* (/ (`self.X or Y`) 2) (`self.Size`))) (`KismetMathLibrary.Conv_IntToDouble` (* (/ (`self.X or Y`) 2) (`self.Size`))))))

(fn `Empty Conditions`
  (params (Index :type Integer))
  (returns (Bool :type Boolean))
  (locals (Index_Local :type Integer))
  (bind (_x__y_x _x__y_y) (`KismetMathLibrary.BreakVector2D` (`self.X, Y`)))
  (bind _x__y_x_2 (`KismetMathLibrary.BreakVector2D` (`self.X, Y`)))
  (bind (_x__y_x_3 _x__y_y_2) (`KismetMathLibrary.BreakVector2D` (`self.X, Y`)))
  (bind (_x__y_x_4 _x__y_y_3) (`KismetMathLibrary.BreakVector2D` (`self.X, Y`)))
  (bind _x__y_x_5 (`KismetMathLibrary.BreakVector2D` (`self.X, Y`)))
  (bind _x__y_x_6 (`KismetMathLibrary.BreakVector2D` (`self.X, Y`)))
  (bind _x__y_x_7 (`KismetMathLibrary.BreakVector2D` (`self.X, Y`)))
  (bind (_x__y_x_8 _x__y_y_4) (`KismetMathLibrary.BreakVector2D` (`self.X, Y`)))
  (bind (_x__y_x_9 _x__y_y_5) (`KismetMathLibrary.BreakVector2D` (`self.X, Y`)))
  (bind _x__y_x_10 (`KismetMathLibrary.BreakVector2D` (`self.X, Y`)))
  (bind (_x__y_x_11 _x__y_y_6) (`KismetMathLibrary.BreakVector2D` (`self.X, Y`)))
  (bind _x__y_x_12 (`KismetMathLibrary.BreakVector2D` (`self.X, Y`)))
  (bind (_x__y_x_13 _x__y_y_7) (`KismetMathLibrary.BreakVector2D` (`self.X, Y`)))
  (bind _x__y_x_14 (`KismetMathLibrary.BreakVector2D` (`self.X, Y`)))
  (bind (_x__y_x_15 _x__y_y_8) (`KismetMathLibrary.BreakVector2D` (`self.X, Y`)))
  (bind _x__y_x_16 (`KismetMathLibrary.BreakVector2D` (`self.X, Y`)))
  (bind _returnvalue (* (- (`self.X or Y`) 1) (`self.Size`)))
  (set `local.Index_Local` Index)
  (return (or (== _x__y_x_7 0.0) (== _x__y_y_4 0.0) (== _x__y_x_6 _returnvalue) (== _x__y_y _returnvalue) (or (== _x__y_x_10 (* (`KismetMathLibrary.RandomIntegerInRange` 0 (- (/ (`self.X or Y`) (`self.EmptyBorderCoefficient`)) 1)) (`self.Size`))) (== _x__y_y_5 (* (`KismetMathLibrary.RandomIntegerInRange` 0 (- (/ (`self.X or Y`) (`self.EmptyBorderCoefficient`)) 1)) (`self.Size`)))) (or (== _x__y_x_12 (* (`KismetMathLibrary.RandomIntegerInRange` (- (`self.X or Y`) (/ (`self.X or Y`) (`self.EmptyBorderCoefficient`))) (`self.X or Y`)) (`self.Size`))) (== _x__y_y_6 (* (`KismetMathLibrary.RandomIntegerInRange` (- (`self.X or Y`) (/ (`self.X or Y`) (`self.EmptyBorderCoefficient`))) (`self.X or Y`)) (`self.Size`)))) (or (== _x__y_x_14 (* (`KismetMathLibrary.RandomIntegerInRange` 0 (- (/ (`self.X or Y`) (* (`self.EmptyBorderCoefficient`) 2)) 1)) (`self.Size`))) (== _x__y_y_7 (* (`KismetMathLibrary.RandomIntegerInRange` 0 (- (/ (`self.X or Y`) (* (`self.EmptyBorderCoefficient`) 2)) 1)) (`self.Size`)))) (or (== _x__y_x_16 (* (`KismetMathLibrary.RandomIntegerInRange` (- (`self.X or Y`) (/ (`self.X or Y`) (* 2 (`self.EmptyBorderCoefficient`)))) (`self.X or Y`)) (`self.Size`))) (== _x__y_y_8 (* (`KismetMathLibrary.RandomIntegerInRange` (- (`self.X or Y`) (/ (`self.X or Y`) (* 2 (`self.EmptyBorderCoefficient`)))) (`self.X or Y`)) (`self.Size`)))) (or (== _x__y_x_5 (* (`KismetMathLibrary.RandomIntegerInRange` 0 (- (/ (`self.X or Y`) (* (`self.EmptyBorderCoefficient`) 4)) 1)) (`self.Size`))) (== _x__y_y_3 (* (`KismetMathLibrary.RandomIntegerInRange` 0 (- (/ (`self.X or Y`) (* (`self.EmptyBorderCoefficient`) 4)) 1)) (`self.Size`)))) (or (== _x__y_x_2 (* (`KismetMathLibrary.RandomIntegerInRange` (- (`self.X or Y`) (/ (`self.X or Y`) (* 4 (`self.EmptyBorderCoefficient`)))) (`self.X or Y`)) (`self.Size`))) (== _x__y_y_2 (* (`KismetMathLibrary.RandomIntegerInRange` (- (`self.X or Y`) (/ (`self.X or Y`) (* 4 (`self.EmptyBorderCoefficient`)))) (`self.X or Y`)) (`self.Size`)))))))

(fn `SpawnActor`
  (params (In :type "Vector2D Structure"))
  (locals (X_Local :type "Float (double-precision)") (Y_Local :type "Float (double-precision)"))
  (set `local.X_Local` In_X)
  (set `local.Y_Local` In_Y)
  (`self.SpawnPickable` (`KismetMathLibrary.MakeVector2D` (`local.X_Local`) (`local.Y_Local`)))
  (switch `int` (`KismetMathLibrary.RandomIntegerInRange` 0 1)
    (:`0`
      (`AddComponent|NODE_AddChildActorComponent-2` :`RelativeTransform` (`KismetMathLibrary.MakeTransform` (`KismetMathLibrary.MakeVector` (`local.X_Local`) (`local.Y_Local`)))) ; Regular
    )
    (:`1`
      (`AddComponent|NODE_AddChildActorComponent-4` :`RelativeTransform` (`KismetMathLibrary.MakeTransform` (`KismetMathLibrary.MakeVector` (`local.X_Local`) (`local.Y_Local`)))) ; Damage
    )))

(fn `SpawnEmpty`
  (params (In :type "Vector2D Structure"))
  (locals (X_Local :type "Float (double-precision)") (Y_Local :type "Float (double-precision)"))
  (set `local.X_Local` In_X)
  (set `local.Y_Local` In_Y)
  (`AddComponent|NODE_AddChildActorComponent-6` :`RelativeTransform` (`KismetMathLibrary.MakeTransform` (`KismetMathLibrary.MakeVector` (`local.X_Local`) (`local.Y_Local`)))) ; Empty
)

(fn `SpawnPickable`
  (params (In :type "Vector2D Structure"))
  (locals (X_Local :type "Float (double-precision)") (Y_Local :type "Float (double-precision)") (Random_Local :type Integer :default 0))
  (set `local.X_Local` In_X)
  (set `local.Y_Local` In_Y)
  (set `local.Random_Local` (`KismetMathLibrary.RandomIntegerInRange` 1 100))
  (if (`KismetMathLibrary.InRange_IntInt` (`local.Random_Local`) 1 3)
    (`AddComponent|NODE_AddChildActorComponent-9` :`RelativeTransform` (`KismetMathLibrary.MakeTransform` (`KismetMathLibrary.MakeVector` (`local.X_Local`) (`local.Y_Local`))))
    (elif (`KismetMathLibrary.InRange_IntInt` (`local.Random_Local`) 4 4)
      (`AddComponent|NODE_AddChildActorComponent-10` :`RelativeTransform` (`KismetMathLibrary.MakeTransform` (`KismetMathLibrary.MakeVector` (`local.X_Local`) (`local.Y_Local`))))
      (elif (`KismetMathLibrary.InRange_IntInt` (`local.Random_Local`) 5 5)
        (`AddComponent|NODE_AddChildActorComponent-11` :`RelativeTransform` (`KismetMathLibrary.MakeTransform` (`KismetMathLibrary.MakeVector` (`local.X_Local`) (`local.Y_Local`))))))))

(fn `UserConstructionScript`
  (for _index (range (+ (`.Total -1 for Loop` (`self.X or Y to second power`)) 1))
    (set `self.X, Y` (`KismetMathLibrary.MakeVector2D` (`KismetMathLibrary.Conv_IntToDouble` (* (/ _index (`self.X or Y`)) (`self.Size`))) (`KismetMathLibrary.Conv_IntToDouble` (* (mod _index (`self.X or Y`)) (`self.Size`)))))
    (bind _bool (`self.Empty Conditions` _index))
    (if _bool
      (`self.SpawnEmpty` (`self.X, Y`)) ; Empty
      (else
        (`KismetArrayLibrary.Array_Add` (`self.NotEmptySquaresArray`) (`self.X, Y`))
        (`self.SpawnActor` (`self.X, Y`))))))

(fn `X or Y to second power`
  (returns (Total :type Integer) (`Total -1 for Loop` :type Integer))
  (bind _x_or_y (`self.X or Y`))
  (bind _returnvalue (* _x_or_y _x_or_y))
  (bind _output_get (set `self.TotalSquares` _returnvalue))
  (return _output_get (- _returnvalue 1)))