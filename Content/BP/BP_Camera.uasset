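; Player camera actor that becomes the view target, follows BP_Character and tilts on input within angle limits.
; Pitch drives the spring arm socket's X offset through trigonometry at a set height.
; The player controller's move event triggers a timeline that lerps the actor's location.
; Tick line-traces toward the character, easing pitch to the AngleLimits.Y extreme when BP_Square_Empty blocks, then back to the saved angle once clear.
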(event `InputAxis|Camera Angle 1`
  (params (AxisValue :type "Float (single-precision)"))
  (bind _angle_limits_x (`KismetMathLibrary.BreakVector2D` (`self.Angle Limits`)))
  (bind _returnvalue (+ (`self.Y Rotation (Pitch)`) AxisValue))
  ;[0.08 0.08 0.08] Change Camera Angle
  (`/Engine/EditorBlueprintResources/StandardMacros.Gate` true :!label _label ; open if pressed\nclose if released
    (:`Exit`
      (if (`PlayerController.IsInputKeyDown` (`self.PlayerController_Ref`) (stale `InputAction|Camera Angle 1` Key))
        (if (not (>= _returnvalue _angle_limits_x))
          (bind _output_get (set `self.Y Rotation (Pitch)` _returnvalue))
          (set `self.Saved Y Rotation ` _output_get)
          (`KismetSystemLibrary.PrintString` (`KismetStringLibrary.Conv_DoubleToString` _output_get) true true (struct :`G` 1.0 :`B` 0.034456 :`A` 1.0) 10.0) ; green
          (`self.FindSidesForCamera x=z*sinX/sinZ`))))))

(event `InputAction|Camera Angle 1`
  (params (Key :type "Key Structure"))
  ;[0.08 0.08 0.08] Change Camera Angle
  (:`Pressed`
    (goto _label :!via `Open`))
  (:`Released`
    (goto _label :!via `Close`)))

(event `InputAxis|Camera Angle 2`
  (params (AxisValue :type "Float (single-precision)"))
  (bind (_angle_limits_x _angle_limits_y) (`KismetMathLibrary.BreakVector2D` (`self.Angle Limits`)))
  (bind _returnvalue (+ (`self.Y Rotation (Pitch)`) AxisValue))
  ;[0.08 0.08 0.08] Change Camera Angle
  (`/Engine/EditorBlueprintResources/StandardMacros.Gate` true :!label _label_2 ; open if pressed\nclose if released
    (:`Exit`
      (if (`PlayerController.IsInputKeyDown` (`self.PlayerController_Ref`) (stale `InputAction|Camera Angle 2` Key))
        (if (not (<= _returnvalue _angle_limits_y))
          (bind _output_get (set `self.Y Rotation (Pitch)` _returnvalue))
          (set `self.Saved Y Rotation ` _output_get)
          (`KismetSystemLibrary.PrintString` (`KismetStringLibrary.Conv_DoubleToString` _output_get) true true (struct :`G` 1.0 :`B` 0.034456 :`A` 1.0) 10.0) ; green
          (`self.FindSidesForCamera x=z*sinX/sinZ`))))))

(event `InputAction|Camera Angle 2`
  (params (Key :type "Key Structure"))
  ;[0.08 0.08 0.08] Change Camera Angle
  (:`Pressed`
    (goto _label_2 :!via `Open`))
  (:`Released`
    (goto _label_2 :!via `Close`)))

(event `self.ReceiveBeginPlay`
  (`self.Set_PlayerController_Ref`)
  (`self.Set_Character_Ref`)
  (add `/Game/BP/BP_PlayerController.MoveButtonsEvent` (`self.PlayerController_Ref`) (`|CreateDelegate` :!event `MoveButtonsEvent`))
  (`PlayerController.SetViewTargetWithBlend` (`self.PlayerController_Ref`) self 0.0 "VTBlend_Linear" 0.0 false) ; Set Camera
  (`self.K2_SetActorLocation` (`self.K2_GetActorLocation` (`self.Character_Ref`))) ; Set Start Location
  (`self.FindSidesForCamera x=z*sinX/sinZ` :!pinned true) ; Angle
)

(event `MoveButtonsEvent`
  (params (x :type "Float (double-precision)") (y :type "Float (double-precision)") (`Rotation Yaw` :type "Float (double-precision)") (Index :type Integer))
  (`self.MoveLocationEvent`))

(event `self.ReceiveTick`
  (params (DeltaSeconds :type "Float (single-precision)"))
  (`self.ObstacleRotationEvent`))

(event `MoveLocationEvent`
  (if (`self.IsLocAnimFinished`)
    (set `self.IsLocAnimFinished` false)
    (bind (_direction _0_to_1) (`Timeline|Timeline_0` :!via `PlayFromStart`)
      (:`Update`
        (set `self.IsLocAnimFinished` false)
        (if (> _0_to_1 0.5)
          (set `self.IsLocAnimFinished` true) ; Finished
          (else
            (`self.K2_SetActorLocation` (`KismetMathLibrary.VLerp` (`SceneComponent.K2_GetComponentLocation` (`self.SpringArm`)) (`self.K2_GetActorLocation` (`self.Character_Ref`)) _0_to_1))))))))

(event `ObstacleRotationEvent`
  (bind (_angle_limits_x _angle_limits_y) (`KismetMathLibrary.BreakVector2D` (`self.Angle Limits`)))
  (bind (_angle_limits_x_2 _angle_limits_y_2) (`KismetMathLibrary.BreakVector2D` (`self.Angle Limits`)))
  (if (`self.IsRotAnimFinished`)
    (if (`self.IsMaxAngle`)
      (bind _isobstacle (`self.LT_IsObstacle`)) ; shoot a linetrace
      (if _isobstacle
        (set `self.IsRotAnimFinished` true)
        (set `self.IsMaxAngle` true)
        (else
          (set `self.IsRotAnimFinished` false)
          (bind (_direction _0_to_1) (`Timeline|Timeline_2` :!via `PlayFromStart`)
            (:`Update`
              (set `self.Y Rotation (Pitch)` (`KismetMathLibrary.Lerp` _angle_limits_y (`self.Saved Y Rotation `) _0_to_1))
              (`self.FindSidesForCamera x=z*sinX/sinZ`)
              (set `self.IsRotAnimFinished` false))
            (:`Finished`
              (set `self.IsRotAnimFinished` true)
              (set `self.IsMaxAngle` false)))))
      (else
        (bind _isobstacle_2 (`self.LT_IsObstacle`)) ; shoot a linetrace
        (if _isobstacle_2
          (set `self.IsRotAnimFinished` false)
          (bind (_direction_2 _0_to_1_2) (`Timeline|Timeline_1` :!via `PlayFromStart`)
            (:`Update`
              (set `self.Y Rotation (Pitch)` (`KismetMathLibrary.Lerp` (`self.Saved Y Rotation `) _angle_limits_y_2 _0_to_1_2))
              (`self.FindSidesForCamera x=z*sinX/sinZ`)
              (set `self.IsRotAnimFinished` false))
            (:`Finished`
              (set `self.IsRotAnimFinished` true)
              (set `self.IsMaxAngle` true)))
          (else
            (set `self.IsRotAnimFinished` true)
            (set `self.IsMaxAngle` false)))))))

(fn `FindAngleForCamera tan(Z) = z/x`
  (bind (_returnvalue_roll _returnvalue_pitch _returnvalue_yaw) (`KismetMathLibrary.BreakRotator` (`SceneComponent.K2_GetComponentRotation` (`self.Camera`))))
  (bind _returnvalue (* (`self.Y Rotation (Pitch)`) -1.0))
  (bind (_socketoffset_x _socketoffset_y) (`KismetMathLibrary.BreakVector` (`SpringArmComponent.SocketOffset` (`self.SpringArm`))))
  (set `SpringArmComponent.SocketOffset` (`KismetMathLibrary.MakeVector` (`self.X Location`) _socketoffset_y (`self.Z Location`)) (`self.SpringArm`))
  (set `self.Y Rotation (Pitch)` (`KismetMathLibrary.DegAtan2` (`KismetMathLibrary.Abs` (`self.Z Location`)) (`KismetMathLibrary.Abs` (`self.X Location`))))
  (`SceneComponent.K2_SetWorldRotation` (`self.Camera`) (`KismetMathLibrary.MakeRotator` _returnvalue_roll _returnvalue _returnvalue_yaw) false false)
  (`KismetSystemLibrary.PrintString` (`KismetStringLibrary.Conv_DoubleToString` _returnvalue) true true (struct :`R` 1.0 :`B` 0.379183 :`A` 1.0) 10.0))

(fn `FindSidesForCamera x=z*sinX/sinZ`
  (bind (_returnvalue_roll _returnvalue_pitch _returnvalue_yaw) (`KismetMathLibrary.BreakRotator` (`SceneComponent.K2_GetComponentRotation` (`self.Camera`))))
  (bind (_socketoffset_x _socketoffset_y) (`KismetMathLibrary.BreakVector` (`SpringArmComponent.SocketOffset` (`self.SpringArm`))))
  (bind _returnvalue (/ (* (`self.Z Location`) (`KismetMathLibrary.DegSin` (- (+ (`KismetMathLibrary.Abs` (`self.Y Rotation (Pitch)`)) 90.0) 180.0))) (`KismetMathLibrary.DegSin` (`KismetMathLibrary.Abs` (`self.Y Rotation (Pitch)`)))))
  (`SceneComponent.K2_SetWorldRotation` (`self.Camera`) (`KismetMathLibrary.MakeRotator` _returnvalue_roll (`self.Y Rotation (Pitch)`) _returnvalue_yaw) false false)
  (set `self.X Location` _returnvalue)
  (set `SpringArmComponent.SocketOffset` (`KismetMathLibrary.MakeVector` (`self.X Location`) _socketoffset_y (`self.Z Location`)) (`self.SpringArm`)) ; Socket offset
  (`KismetSystemLibrary.PrintString` (`KismetStringLibrary.Conv_DoubleToString` _returnvalue) true true (struct :`R` 1.0 :`B` 0.379183 :`A` 1.0) 10.0))

(fn `LT_IsObstacle`
  (returns (IsObstacle :type Boolean))
  (locals (`Remembered Degree_Local` :type "Float (double-precision)"))
  (bind (_returnvalue_x _returnvalue_y _returnvalue_z) (`KismetMathLibrary.BreakVector` (`self.K2_GetActorLocation` (`self.Character_Ref`))))
  (bind (_returnvalue_x_2 _returnvalue_y_2 _returnvalue_z_2) (`KismetMathLibrary.BreakVector` (`SceneComponent.K2_GetComponentLocation` (`self.LT Camera`))))
  (bind (_outhit _returnvalue) (`KismetSystemLibrary.LineTraceSingle` :`Start` (`KismetMathLibrary.MakeVector` _returnvalue_x_2 _returnvalue_y_2 (- _returnvalue_z_2 0.0)) :`End` (`KismetMathLibrary.MakeVector` (- _returnvalue_x 45.0) _returnvalue_y _returnvalue_z) :`TraceChannel` "TraceTypeQuery1" :`DrawDebugType` "ForDuration" :`TraceColor` (struct :`R` 0.483395 :`B` 1.0 :`A` 1.0) :`DrawTime` 2.0))
  (bind _returnvalue_2 (`GameplayStatics.GetObjectClass` (`.HitActor` (`GameplayStatics.BreakHitResult` _outhit))))
  (return (and (!= _returnvalue_2 "/Game/BP/BP_Character.BP_Character_C") (== _returnvalue_2 "/Game/BP/Square/BP_Square_Empty.BP_Square_Empty_C") _returnvalue)))

(fn `Set_Character_Ref`
  (`/Engine/EditorBlueprintResources/StandardMacros.IsValid` (`self.Character_Ref`)
    (:`Is Not Valid`
      (bind _returnvalue (`GameplayStatics.GetActorOfClass` "/Game/BP/BP_Character.BP_Character_C"))
      (set `self.Character_Ref` _returnvalue))))

(fn `Set_PlayerController_Ref`
  (`/Engine/EditorBlueprintResources/StandardMacros.IsValid` (`self.PlayerController_Ref`)
    (:`Is Not Valid`
      (bind _asbp_player_controller (cast `/Game/BP/BP_PlayerController` (`GameplayStatics.GetPlayerController` 0)))
      (set `self.PlayerController_Ref` _asbp_player_controller))))

(fn `UserConstructionScript`)