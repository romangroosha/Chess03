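; BP_AI_Enemy is a board-game enemy, still partly wired, that detects BP_Character through a search collision and labels itself with its instance suffix.
; It caches game references and binds to the player controller's move-button event.
; Once the character is sighted, each move event line-traces surrounding offsets to rebuild ActorsAround from non-empty squares and the character.
; Relocation and square-lighting logic is never run, and move/lerp helpers are not called here.
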(event `self.ReceiveBeginPlay`
  (`self.Set_GameMode_Ref`)
  (`self.Set_Character_Ref`)
  (`self.Set_Board_Ref`)
  (`self.Set_PlayerController_Ref`)
  (`self.Set_Camera_Ref`)
  (add `/Game/BP/BP_PlayerController.MoveButtonsEvent` (`self.PlayerController_Ref`) (`|CreateDelegate` :!event `Move Buttons Event`))
  (bind _returnvalue (`AddComponent|NODE_AddTextRenderComponent-0`))
  (`TextRenderComponent.K2_SetText` _returnvalue (`KismetTextLibrary.Conv_StringToText` (`.RightS` (`KismetStringLibrary.Split` (`KismetSystemLibrary.GetDisplayName` self) "BP_AI_Enemy_C_")))))

(event `Move Buttons Event`
  (params (x :type "Float (double-precision)") (y :type "Float (double-precision)") (`Rotation Yaw` :type "Float (double-precision)") (Index :type Integer))
  (if (`self.IsCharInSight`)
    (`self.LT_MakeActorsArround`)))

(event `self.EnemyCollision.OnComponentBeginOverlap`
  (params (OverlappedComponent :type "PrimitiveComponent Object Reference") (OtherActor :type "Actor Object Reference") (OtherComp :type "PrimitiveComponent Object Reference") (OtherBodyIndex :type Integer) (bFromSweep :type Boolean) (SweepResult :type "HitResult Structure (by ref)"))
  (if (== OtherActor (`self.Character_Ref`))
    _))

(event `self.SearchCollision.OnComponentBeginOverlap`
  (params (OverlappedComponent :type "PrimitiveComponent Object Reference") (OtherActor :type "Actor Object Reference") (OtherComp :type "PrimitiveComponent Object Reference") (OtherBodyIndex :type Integer) (bFromSweep :type Boolean) (SweepResult :type "HitResult Structure (by ref)"))
  (if (== OtherActor (`self.Character_Ref`))
    (set `self.IsCharInSight` true)))

(fn `LerpLocation_Move`
  (params (Alpha :type "Float (double-precision)"))
  (locals (NewLocalVar_0 :type "Vector Structure") (NewLocalVar_1 :type "Vector Structure"))
  (`self.K2_SetActorLocation` (`KismetMathLibrary.VLerp` (`self.Move_Location 1`) (`self.Move_Location 2`) Alpha)))

(fn `LerpRotation_Move`
  (params (Alpha :type "Float (double-precision)") (`Set Target` :type "SceneComponent Object Reference"))
  (locals (Set_Target_Local :type "SceneComponent Object Reference"))
  (set `local.Set_Target_Local` `Set Target`)
  (if (!= (`self.Move_Rotation 1`) (`self.Move_Rotation 2`))
    (if (and (or (== (`self.Move_Rotation 1`) 180.0) (== (`self.Move_Rotation 1`) 135.0)) (`KismetMathLibrary.InRange_FloatFloat` (`self.Move_Rotation 2`) -135.0 -45.0))
      (set `self.Move_Rotation 2` (+ (`self.Move_Rotation 2`) 360.0))
      (elif (and (`KismetMathLibrary.InRange_FloatFloat` (`self.Move_Rotation 1`) -135.0 -45.0) (or (== (`self.Move_Rotation 2`) 180.0) (== (`self.Move_Rotation 2`) 135.0)))
        (set `self.Move_Rotation 2` (- (`self.Move_Rotation 2`) 360.0))))
    (`SceneComponent.K2_SetWorldRotation` (`local.Set_Target_Local`) (`KismetMathLibrary.MakeRotator` 0.0 0.0 (`KismetMathLibrary.Lerp` (`self.Move_Rotation 1`) (`self.Move_Rotation 2`) Alpha)) false false)))

(fn `LT_MakeActorsArround`
  (locals (ObjectTypes :type "Array of EObjectTypeQuery Enum"))
  (`KismetArrayLibrary.Array_Clear` (`self.ActorsAround`))
  (for _array_element (`self.LocationsAround`)
    (bind (_outhit _returnvalue) (`KismetSystemLibrary.LineTraceSingleForObjects` :`Start` (`SceneComponent.K2_GetComponentLocation` (`self.LT_EnemySphere`)) :`End` (+ (`KismetMathLibrary.MakeVector` (`KismetMathLibrary.BreakVector2D` _array_element) (`.Y` (`KismetMathLibrary.BreakVector2D` _array_element)) -25.0) (`self.K2_GetActorLocation`)) :`ObjectTypes` (`local.ObjectTypes`) :`TraceColor` (struct :`R` 1.0 :`G` 0.503061 :`A` 1.0)))
    (bind _returnvalue_2 (`GameplayStatics.GetObjectClass` (`.HitActor` (`GameplayStatics.BreakHitResult` _outhit))))
    (if (or (and (`KismetMathLibrary.ClassIsChildOf` _returnvalue_2 "/Script/Engine.Character") (== _returnvalue_2 "/Game/BP/BP_Character.BP_Character_C")) (and (`KismetMathLibrary.ClassIsChildOf` (`GameplayStatics.GetObjectClass` (`.HitActor` (`GameplayStatics.BreakHitResult` _outhit))) "/Game/BP/BP_Square.BP_Square_C") (!= (`GameplayStatics.GetObjectClass` (`.HitActor` (`GameplayStatics.BreakHitResult` _outhit))) "/Game/BP/Square/BP_Square_Empty.BP_Square_Empty_C") _returnvalue))
      (`KismetArrayLibrary.Array_Add` (`self.ActorsAround`) (`.HitActor` (`GameplayStatics.BreakHitResult` _outhit))))))

(fn `LT_Move`
  (returns (Bool :type Boolean))
  (locals (X_Local :type "Float (double-precision)") (Y_Local :type "Float (double-precision)") (IndexRotation_Local :type "Float (double-precision)") (ObjectTypes_Local :type "Array of EObjectTypeQuery Enum"))
  (bind _outhit (`KismetSystemLibrary.LineTraceSingleForObjects` (`SceneComponent.K2_GetComponentLocation` (`self.LT_EnemySphere`)) (+ (`KismetMathLibrary.MakeVector` (`self.Move_X`) (`self.Move_Y`) -25.0) (`self.K2_GetActorLocation`)) (`local.ObjectTypes_Local`))) ; Line Traces from LT_Sphere to Move Location
  (return (and (`KismetMathLibrary.ClassIsChildOf` (`GameplayStatics.GetObjectClass` (`.HitActor` (`GameplayStatics.BreakHitResult` _outhit))) "/Game/BP/BP_Square.BP_Square_C") (!= (`GameplayStatics.GetObjectClass` (`.HitActor` (`GameplayStatics.BreakHitResult` _outhit))) "/Game/BP/Square/BP_Square_Empty.BP_Square_Empty_C"))))

(fn `Set_Board_Ref`
  (`/Engine/EditorBlueprintResources/StandardMacros.IsValid` (`self.Board_Ref`)
    (:`Is Not Valid`
      (bind _returnvalue (`GameplayStatics.GetActorOfClass` "/Game/BP/BP_Board.BP_Board_C"))
      (set `self.Board_Ref` _returnvalue))))

(fn `Set_Camera_Ref`
  (`/Engine/EditorBlueprintResources/StandardMacros.IsValid` (`self.Camera_Ref`)
    (:`Is Not Valid`
      (bind _returnvalue (`GameplayStatics.GetActorOfClass` "/Game/BP/BP_Camera.BP_Camera_C"))
      (set `self.Camera_Ref` _returnvalue))))

(fn `Set_CameraStartLocation`
  (locals (`Save Camera Lag Status` :type Boolean))
  (set `local.Save Camera Lag Status` (`SpringArmComponent.bEnableCameraLag` (`/Game/BP/BP_Camera.SpringArm` (`self.Camera_Ref`))))
  (set `SpringArmComponent.bEnableCameraLag` false (`/Game/BP/BP_Camera.SpringArm` (`self.Camera_Ref`)))
  (`self.K2_SetActorLocation` (`self.Camera_Ref`) (`KismetMathLibrary.MakeVector` (- (.x (`self.K2_GetActorLocation`)) 400.0) (.y (`self.K2_GetActorLocation`)) (+ (.z (`self.K2_GetActorLocation`)) 1000.0)) false false) ; Set Start Location
  (set `SpringArmComponent.bEnableCameraLag` (`local.Save Camera Lag Status`) (`/Game/BP/BP_Camera.SpringArm` (`self.Camera_Ref`))))

(fn `Set_Character_Ref`
  (`/Engine/EditorBlueprintResources/StandardMacros.IsValid` (`self.Character_Ref`)
    (:`Is Not Valid`
      (bind _returnvalue (`GameplayStatics.GetActorOfClass` "/Game/BP/BP_Character.BP_Character_C"))
      (set `self.Character_Ref` _returnvalue))))

(fn `Set_GameMode_Ref`
  (`/Engine/EditorBlueprintResources/StandardMacros.IsValid` (`self.GameMode_Ref`)
    (:`Is Not Valid`
      (bind _returnvalue (`GameplayStatics.GetActorOfClass` "/Game/BP/BP_GameMode.BP_GameMode_C"))
      (set `self.GameMode_Ref` _returnvalue))))

(fn `Set_MoveUtilityVariables`
  (params (`Set Target` :type "SceneComponent Object Reference"))
  (bind _returnvalue (`self.K2_GetActorLocation`))
  (bind (_returnvalue_roll _returnvalue_pitch _returnvalue_yaw) (`KismetMathLibrary.BreakRotator` (`SceneComponent.K2_GetComponentRotation` `Set Target`)))
  (set `self.Move_Location 1` _returnvalue)
  (set `self.Move_Location 2` (+ (`KismetMathLibrary.MakeVector` (`self.Move_X`) (`self.Move_Y`)) _returnvalue))
  (set `self.Move_Rotation 1` _returnvalue_yaw)
  (set `self.Move_Rotation 2` (`self.Move_Rotation Yaw`)))

(fn `Set_MoveVariables`
  (params (x :type "Float (double-precision)") (y :type "Float (double-precision)") (`Rotation Yaw` :type "Float (double-precision)") (index :type Integer))
  (set `self.Move_X` x)
  (set `self.Move_Y` y)
  (set `self.Move_Rotation Yaw` `Rotation Yaw`)
  (set `self.Move_Index` index))

(fn `Set_NewLocationForEnemy`
  (params (`New Location Z` :type "Float (double-precision)"))
  (locals (ArrayElement_Local :type "Actor Object Reference") (Counter_Local :type Integer) (IsGreater2 :type Boolean))
  (bind (_returnvalue_x _returnvalue_y) (`KismetMathLibrary.BreakVector` (`self.K2_GetActorLocation` (`local.ArrayElement_Local`))))
  (`KismetArrayLibrary.Array_Clear` (`/Game/BP/BP_GameMode.CrossoversEnemy` (`self.GameMode_Ref`)))
  (for _array_element (`self.ActorsAround`)
    (set `local.ArrayElement_Local` _array_element)
    (set `self.IsEnemyLocFound` false)
    (if (== (`self.K2_GetActorLocation` (`local.ArrayElement_Local`)) (`self.K2_GetActorLocation` (`self.Character_Ref`)) :`ErrorTolerance` 200.0)
      (set `self.IsEnemyLocFound` true)
      (`KismetArrayLibrary.Array_Add` (`/Game/BP/BP_GameMode.CrossoversEnemy` (`self.GameMode_Ref`)) (`self.K2_GetActorLocation` (`local.ArrayElement_Local`)))
      (break)))
  (if (`self.IsEnemyLocFound`)
    (set `local.Counter_Local` 0)
    (for _array_element_2 (`/Game/BP/BP_GameMode.CrossoversEnemy` (`self.GameMode_Ref`))
      (set `local.IsGreater2` false)
      (if (== _array_element_2 (`self.K2_GetActorLocation` (`local.ArrayElement_Local`)))
        (bind _result (`/Engine/EditorBlueprintResources/StandardMacros.IncrementInt` (`local.Counter_Local`))
          (:`  `
            (set `local.IsGreater2` false)
            (if (>= _result 2)
              (set `local.IsGreater2` true)
              (break))))))
    (if (`local.IsGreater2`)
      (`self.K2_SetActorLocation` (`KismetMathLibrary.MakeVector` _returnvalue_x _returnvalue_y `New Location Z`)))))

(fn `Set_PlayerController_Ref`
  (`/Engine/EditorBlueprintResources/StandardMacros.IsValid` (`self.PlayerController_Ref`)
    (:`Is Not Valid`
      (bind _asbp_player_controller (cast `/Game/BP/BP_PlayerController` (`GameplayStatics.GetPlayerController` 0)))
      (set `self.PlayerController_Ref` _asbp_player_controller))))

(fn `UserConstructionScript`)

(fn `WhichDirectionCharIsLooking_Move`
  (params (`Set Target` :type "StaticMeshComponent Object Reference"))
  (locals (SetTarget_Local :type "StaticMeshComponent Object Reference"))
  (set `local.SetTarget_Local` `Set Target`)
  (bind _keys (`BlueprintMapLibrary.Map_Keys` (`self.Move_DirectionMap`)))
  (for _array_element _keys
    (if (== _array_element (`SceneComponent.GetForwardVector` (`local.SetTarget_Local`)) :`ErrorTolerance` 0.1)
      (set `self.Move_Direction` (`BlueprintMapLibrary.Map_Find` (`self.Move_DirectionMap`) _array_element))
      (break)))
  (return))