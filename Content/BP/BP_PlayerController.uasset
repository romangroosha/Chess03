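; Player controller that turns keyboard input into four-way movement commands, blocking reversal of the character's current direction.
; BeginPlay caches a BP_Character reference, whose MoveDirection gates each press from WASD, arrow or numpad keys.
; Allowed presses call MoveButtonsEvent with an axis offset, yaw and direction index.
; Four diagonal variants are present but unconnected to any input.
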(event `self.ReceiveBeginPlay`
  (`self.Set_Character_Ref`))

(event `Key|NumPadSeven`
  (params (Key :type "Key Structure")))

(event `Key|NumPadEight`
  (params (Key :type "Key Structure")))

(event `Key|NumPadNine`
  (params (Key :type "Key Structure")))

(event `Key|NumPadFour`
  (params (Key :type "Key Structure")))

(event `Key|NumPadSix`
  (params (Key :type "Key Structure")))

(event `Key|S`
  (params (Key :type "Key Structure"))
  (bind _move_direction (`/Game/BP/BP_Character.Move_Direction` (`self.Character_Ref`)))
  (:`Pressed`
    (if (or (== _move_direction "D") (== _move_direction "R") (== _move_direction "L")) :!label _label
      (`self.MoveButtonsEvent` -100.0 :!pinned true) ; down
    )))

(event `Key|NumPadTwo`
  (params (Key :type "Key Structure"))
  (:`Pressed`
    (goto _label)))

(event `Key|Down`
  (params (Key :type "Key Structure"))
  (:`Pressed`
    (goto _label)))

(event `Key|A`
  (params (Key :type "Key Structure"))
  (bind _move_direction (`/Game/BP/BP_Character.Move_Direction` (`self.Character_Ref`)))
  (:`Pressed`
    (if (or (== _move_direction "U") (== _move_direction "D") (== _move_direction "L")) :!label _label_2
      (`self.MoveButtonsEvent` 0.0 -100.0 90.0 2 :!pinned true) ; left
    )))

(event `Key|NumPadOne`
  (params (Key :type "Key Structure"))
  (:`Pressed`
    (goto _label_2)))

(event `Key|Left`
  (params (Key :type "Key Structure"))
  (:`Pressed`
    (goto _label_2)))

(event `Key|W`
  (params (Key :type "Key Structure"))
  (bind _move_direction (`/Game/BP/BP_Character.Move_Direction` (`self.Character_Ref`)))
  (:`Pressed`
    (if (or (== _move_direction "U") (== _move_direction "L") (== _move_direction "R")) :!label _label_3
      (`self.MoveButtonsEvent` 100.0 0.0 180.0 4 :!pinned true) ; up
    )))

(event `Key|NumPadFive`
  (params (Key :type "Key Structure"))
  (:`Pressed`
    (goto _label_3)))

(event `Key|Up`
  (params (Key :type "Key Structure"))
  (:`Pressed`
    (goto _label_3)))

(event `Key|D`
  (params (Key :type "Key Structure"))
  (bind _move_direction (`/Game/BP/BP_Character.Move_Direction` (`self.Character_Ref`)))
  (:`Pressed`
    (if (or (== _move_direction "U") (== _move_direction "D") (== _move_direction "R")) :!label _label_4
      (`self.MoveButtonsEvent` 0.0 100.0 -90.0 6 :!pinned true) ; right
    )))

(event `Key|NumPadThree`
  (params (Key :type "Key Structure"))
  (:`Pressed`
    (goto _label_4)))

(event `Key|Right`
  (params (Key :type "Key Structure"))
  (:`Pressed`
    (goto _label_4)))

(fn `Set_Character_Ref`
  (`/Engine/EditorBlueprintResources/StandardMacros.IsValid` (`self.Character_Ref`)
    (:`Is Not Valid`
      (bind _returnvalue (`GameplayStatics.GetActorOfClass` "/Game/BP/BP_Character.BP_Character_C"))
      (set `self.Character_Ref` _returnvalue))))

(fn `UserConstructionScript`)